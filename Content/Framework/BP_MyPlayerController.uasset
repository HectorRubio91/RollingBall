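; Player controller that owns the main HUD and shows the player's lives and score.
; On BeginPlay it creates WBP_MainWidget, adds it to the viewport and fills in the current lives and score.
; UpdateUILives and UpdateUIScore events pass new values to helper functions that write labelled text straight into the widget's LivesText and ScoreText fields.
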(event EventBeginPlay
  ;[0.15 0.15 0.15 0.5] Aniadir UI del score y vidas
  (CallFunction|InitWidget)
  (CallFunction|SetUILives (Variables|Default|GetCurrentLives))
  (CallFunction|SetUIScore (Variables|Default|GetCurrentScore)))

(event EventUpdateUIScore
  (params (NewScore :type Integer))
  ;[0.15 0.15 0.15 0.5] Actualizar score
  (CallFunction|SetUIScore NewScore))

(event EventUpdateUILives
  (params (NewLives :type Integer))
  ;[0.15 0.15 0.15 0.5] Actualizar vidas en el UI
  (CallFunction|SetUILives NewLives))

(fn ConstructionScript)

(fn InitWidget
  (bind _returnvalue (UserInterface|CreateWidget "/Game/UI/WBP_MainWidget.WBP_MainWidget_C" self))
  (bind _output_get (Variables|Default|SetMainWidget _returnvalue))
  (UserInterface|Viewport|AddtoViewport _output_get 0))

(fn SetUILives
  (params (Lives :type Integer))
  (Rendering|Components|TextRender|SetText (Variables|/Game/UI/WBP_MainWidget.WBP_MainWidget_C|GetLivesText (Variables|Default|GetMainWidget)) (Utilities|Text|ToText(String) (Utilities|String|Append "Lives: " (Utilities|String|ToString(Integer) Lives)))))

(fn SetUIScore
  (params (Score :type Integer))
  (Rendering|Components|TextRender|SetText (Variables|/Game/UI/WBP_MainWidget.WBP_MainWidget_C|GetScoreText (Variables|Default|GetMainWidget)) (Utilities|Text|ToText(String) (Utilities|String|Append "Score: " (Utilities|String|ToString(Integer) Score)))))